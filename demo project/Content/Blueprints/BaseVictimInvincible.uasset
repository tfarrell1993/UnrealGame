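; BaseVictimInvincible is a fleeing target that rewards the physics ball with an invincibility upgrade when worn down.
; Tick moves it away from the player within range by setting location without sweep, faster as distance grows.
; Ball hits shrink it until, below a scale threshold, a hit heals the ball, grants invincibility and sets a checkpoint.
; It then spawns a respawn marker, passes it to the player's ball and destroys itself.
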(event EventTick
  (params (DeltaSeconds :type Float%20%28single-precision%29))
  (bind _returnvalue (Game|Player|GetPlayerPawn 0))
  (bind _returnvalue_2 (Transformation|GetActorLocation))
  ;[1 1 1] See if close enough to player
  (bind _returnvalue_3 (Transformation|GetDistanceTo _returnvalue))
  (if (<= _returnvalue_3 1e+03)
    (Transformation|SetActorLocation (+ _returnvalue_2 (* (* (- _returnvalue_2 (Transformation|GetActorLocation _returnvalue)) DeltaSeconds) 0.3)) false)))

(event EventHit
  (params (MyComp :type Primitive%20Component%20Object%20Reference) (Other :type Actor%20Object%20Reference) (OtherComp :type Primitive%20Component%20Object%20Reference) (bSelfMoved :type Boolean) (HitLocation :type Vector :default "0, 0, 0") (HitNormal :type Vector :default "0, 0, 0") (NormalImpulse :type Vector :default "0, 0, 0") (Hit :type Hit%20Result%20Structure%20%28by%20ref%29))
  (bind _returnvalue (Transformation|GetActorScale3D))
  (bind (_x _y _z) (Math|Vector|BreakVector _returnvalue))
  ;[1 1 1] Upgrade
  (bind _asphysicsballbp_c (Utilities|Casting|CastToPhysicsBallBP Other))
  (if (< (.X (Math|Vector|BreakVector _returnvalue)) 0.3)
    (Default|HealDamage _asphysicsballbp_c)
    (Default|UPInvincible _asphysicsballbp_c)
    (Default|SetCheckpoint _asphysicsballbp_c true)
    (bind _returnvalue_2 (Game|SpawnActorfromClass "/Game/Blueprints/RespawnMarker.RespawnMarker_C" (Math|Conversions|ToTransform(Vector) HitLocation) true 0))
    (bind _asphysicsballbp_c_2 (Utilities|Casting|CastToPhysicsBallBP (Game|Player|GetPlayerPawn 0))
      (:then
        (Default|StacheActor _asphysicsballbp_c_2 _returnvalue_2))
      (:CastFailed
        _))
    (Actor|DestroyActor)
    (else
      (Transformation|SetActorScale3D (Math|Vector|MakeVector (- (* _x 0.9) 0.05) (- (* _y 0.9) 0.05) (- (* _z 0.9) 0.05))))))

(fn ConstructionScript
  (Variables|Default|SetUpgradeType 0))