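; SeekerBall is a homing hazard actor that chases the player pawn and damages it on contact.
; Each tick it moves straight toward the player at constant speed without sweeping, and destroys itself once the player is out of range.
; A hit on the player after a short arming delay calls TakeDamage on the PhysicsBallBP pawn, then destroys the seeker.
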(event EventTick
  (params (DeltaSeconds :type Float%20%28single-precision%29))
  (bind _returnvalue (Game|Player|GetPlayerPawn 0))
  (bind _returnvalue_2 (Transformation|GetActorLocation))
  (Variables|Default|SetTimePassed (+ (Variables|Default|GetTimePassed) DeltaSeconds))
  (bind _returnvalue_3 (Transformation|GetDistanceTo _returnvalue))
  (if (< _returnvalue_3 1e+03)
    (Transformation|SetActorLocation (+ _returnvalue_2 (* (* (Math|Vector|Normalize (- (Transformation|GetActorLocation _returnvalue) _returnvalue_2)) (+ 0.0 DeltaSeconds)) 2e+02)) false)
    (else
      (Actor|DestroyActor))))

(event EventHit
  (params (MyComp :type Primitive%20Component%20Object%20Reference) (Other :type Actor%20Object%20Reference) (OtherComp :type Primitive%20Component%20Object%20Reference) (bSelfMoved :type Boolean) (HitLocation :type Vector :default "0, 0, 0") (HitNormal :type Vector :default "0, 0, 0") (NormalImpulse :type Vector :default "0, 0, 0") (Hit :type Hit%20Result%20Structure%20%28by%20ref%29))
  (bind _returnvalue (Game|Player|GetPlayerPawn 0))
  (if (== _returnvalue Other)
    (if (> (Variables|Default|GetTimePassed) 2.0)
      (bind _asphysicsballbp_c (Utilities|Casting|CastToPhysicsBallBP _returnvalue))
      (Default|TakeDamage _asphysicsballbp_c)
      (Actor|DestroyActor))))

(fn ConstructionScript)