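; BP_Victim is an actor that the player pawn can carry along by holding Q while nearby.
; Each Tick it checks its distance to player pawn 0 and, when close, prints a debug message and polls the key.
; Holding Q attaches its root component to the pawn, keeping world position; otherwise it detaches, but only while within range.
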(event EventTick
  (params (DeltaSeconds :type Float%20%28single-precision%29))
  ;[1 1 1] Check Player Close
  (bind _returnvalue (Transformation|GetDistanceTo (Game|Player|GetPlayerPawn 0)))
  (if (<= _returnvalue 2e+02)
    (Development|PrintString "Close")
    ;[1 1 1] Check Key Down
    (if (Game|Player|IsInputKeyDown (Game|GetPlayerController 0) "Q")
      ;[1 1 1] Attach/Detach
      (Class|Actor|AttachRootComponenttoActor (Game|Player|GetPlayerPawn 0) "None" "KeepWorldPosition" true)
      (else
        (Class|Actor|DetachRootComponentfromParent true)))))

(fn ConstructionScript)