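; BP_AvoidPlayer is an actor that drifts away from the player pawn when it comes within 1000 units.
; Each tick it measures and prints its distance to player 0, then offsets its location along the unnormalized player-to-actor vector, scaled by delta time and a small factor.
; The push therefore grows with distance inside the range, and the move does not sweep for collision.
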(event EventTick
  (params (DeltaSeconds :type Float%20%28single-precision%29))
  (bind _returnvalue (Transformation|GetActorLocation))
  (bind _returnvalue_2 (Game|Player|GetPlayerPawn 0))
  ;[1 1 1] See if close enough to player
  (bind _returnvalue_3 (Transformation|GetDistanceTo _returnvalue_2))
  (Development|PrintString (Utilities|String|ToString(Float) _returnvalue_3))
  (if (<= _returnvalue_3 1e+03)
    (Transformation|SetActorLocation (+ _returnvalue (* (* (- _returnvalue (Transformation|GetActorLocation _returnvalue_2)) DeltaSeconds) 0.01)) false)))

(fn ConstructionScript)